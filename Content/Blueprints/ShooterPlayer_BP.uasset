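; Player Blueprint for a shooter that owns the game's UI widgets and handles the player's death.
; CECreateUI creates and stores the start menu and HUD widgets without adding them to the viewport.
; CEDeath, guarded by a DoOnce, hides the player mesh, waits briefly, then shows the game-over widget, pauses the game and disables input.
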(event `self.CE_CreateUI`
  (bind _returnvalue (`|CreateWidget` "/Game/Blueprints/W_ShooterGameStart.W_ShooterGameStart_C"))
  (set `self.GameStartMenu` _returnvalue)
  (bind _returnvalue_2 (`|CreateWidget` "/Game/Blueprints/W_HUD.W_HUD_C"))
  (set `self.InGameHUD` _returnvalue_2))

(event `self.CE_Death`
  (`/Engine/EditorBlueprintResources/StandardMacros.DoOnce` false
    (:`Completed`
      (`SceneComponent.SetVisibility` (`self.PlayerMesh`) false true)
      (`KismetSystemLibrary.Delay` 2.0)
      (bind _returnvalue (`|CreateWidget` "/Game/Blueprints/W_ShooterGameOver.W_ShooterGameOver_C"))
      (bind _output_get (set `self.GameOverMenu` _returnvalue))
      (`UserWidget.AddToViewport` _output_get 0)
      (`GameplayStatics.SetGamePaused` true)
      (`self.DisableInput` null))))

(fn `UserConstructionScript`)